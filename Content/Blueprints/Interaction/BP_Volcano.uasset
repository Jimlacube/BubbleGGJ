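; Volcano experiment actor that erupts once it has received both bicarb and vinegar.
; Its Box overlap ignores held items and identifies each ingredient through message calls on the overlapping actor.
; A matching ingredient has physics and collision disabled, attaches to the Box, is told it is attached, and sets its flag.
; With both flags set, it spawns a BP_BubbleSpawner at VolcanoTop and activates the NSVolcano effect.
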(event `self.ReceiveBeginPlay`
  (`self.K2_SetActorLocation` (`KismetMathLibrary.MakeVector` (.x (`self.K2_GetActorLocation`)) 0.0 (.z (`self.K2_GetActorLocation`)))))

(event `self.Box.OnComponentBeginOverlap`
  (params (OverlappedComponent :type "PrimitiveComponent Object Reference") (OtherActor :type "Actor Object Reference") (OtherComp :type "PrimitiveComponent Object Reference") (OtherBodyIndex :type Integer) (bFromSweep :type Boolean) (SweepResult :type "HitResult Structure (by ref)"))
  (bind _return (message `/Game/Blueprints/Objects/BPI_Object.IsHeld` OtherActor))
  (if (not _return)
    (`|ExecutionSequence`
      (:`then_0`
        (bind _return_2 (message `/Game/Blueprints/Objects/BPI_Object.IsBicarb` OtherActor))
        (if _return_2
          (message `/Game/Blueprints/Objects/BPI_Object.SetSimulatePhysics` OtherActor false)
          (message `/Game/Blueprints/Objects/BPI_Object.DisableCollision` OtherActor)
          (`self.K2_AttachToComponent` OtherActor (`self.Box`) "None" "SnapToTarget" "KeepRelative" "KeepRelative" true)
          (message `/Game/Blueprints/Objects/BPI_Object.SetAttachedToVolcano` OtherActor)
          (set `self.BicarbGot` true)
          (if (and (`self.BicarbGot`) (`self.VinegarGot`)) :!label _label
            (`|SpawnActorFromClass` "/Game/Blueprints/Tools/BP_BubbleSpawner.BP_BubbleSpawner_C" (`KismetMathLibrary.MakeTransform` (`SceneComponent.K2_GetComponentLocation` (`self.VolcanoTop`))) "AlwaysSpawn" "MultiplyWithRoot" null 0.1 0.2 null)
            (`ActorComponent.Activate` (`self.NS_Volcano`) false))))
      (:`then_1`
        (bind _return_3 (message `/Game/Blueprints/Objects/BPI_Object.IsVinegar` OtherActor))
        (if _return_3
          (message `/Game/Blueprints/Objects/BPI_Object.SetSimulatePhysics` OtherActor false)
          (message `/Game/Blueprints/Objects/BPI_Object.DisableCollision` OtherActor)
          (`self.K2_AttachToComponent` OtherActor (`self.Box`) "None" "SnapToTarget" "KeepRelative" "KeepRelative" true)
          (message `/Game/Blueprints/Objects/BPI_Object.SetAttachedToVolcano` OtherActor)
          (set `self.VinegarGot` true)
          (goto _label))))))

(fn `UserConstructionScript`)