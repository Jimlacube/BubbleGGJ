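; BP_PlayerBubble is the player-controlled bubble, which moves on the world X-Z plane and spawns other bubbles.
; It registers its Enhanced Input mapping context on BeginPlay and feeds the 2D movement action into AddMovementInput.
; The action input spawns a BP_Bubble at the player's location and launches its sphere in a random direction with a mass-independent impulse.
; The Hit event and construction script are empty.
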(event `self.ReceiveBeginPlay`
  (`EnhancedInputSubsystemInterface.AddMappingContext` (pcsubsystem `EnhancedInputLocalPlayerSubsystem` (`GameplayStatics.GetPlayerController` 0)) "/Game/Input/IMC_MappingContext.IMC_MappingContext" 0 (struct)))

(event `EnhancedInput|/Game/Input/IA_Movement`
  (params (ActionValue :type "Vector2D Structure") (ElapsedSeconds :type "Float (double-precision)") (TriggeredSeconds :type "Float (double-precision)") (InputAction :type "InputAction Object Reference" :default "/Game/Input/IA_Movement.IA_Movement"))
  (bind (_x _y) (`KismetMathLibrary.BreakVector2D` ActionValue))
  (:`Triggered`
    (`self.AddMovementInput` (`KismetMathLibrary.MakeVector` _x 0.0 _y))))

(event `EnhancedInput|/Game/Input/IA_Action`
  (params (ActionValue :type Boolean) (ElapsedSeconds :type "Float (double-precision)") (TriggeredSeconds :type "Float (double-precision)") (InputAction :type "InputAction Object Reference" :default "/Game/Input/IA_Action.IA_Action"))
  (:`Triggered`
    (bind _returnvalue (`|SpawnActorFromClass` "/Game/Blueprints/Projectile/BP_Bubble.BP_Bubble_C" (`KismetMathLibrary.MakeTransform` (`self.K2_GetActorLocation`)) "AlwaysSpawn" "MultiplyWithRoot" null null))
    (`PrimitiveComponent.AddImpulse` (`/Game/Blueprints/Projectile/BP_Bubble.Sphere` _returnvalue) (* (`KismetMathLibrary.RandomUnitVector`) (`self.BubbleSpawnForce`)) "None" true)))

(event `self.ReceiveHit`
  (params (MyComp :type "PrimitiveComponent Object Reference") (Other :type "Actor Object Reference") (OtherComp :type "PrimitiveComponent Object Reference") (bSelfMoved :type Boolean) (HitLocation :type "Vector Structure") (HitNormal :type "Vector Structure") (NormalImpulse :type "Vector Structure") (Hit :type "HitResult Structure (by ref)")))

(fn `UserConstructionScript`)