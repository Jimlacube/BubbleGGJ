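; Game mode that sets up the game's layered ambient audio when play begins.
; It mutes the persistent submix and every room submix, then starts all base soundscapes at once as 2D sounds.
; A timeline then fades the persistent submix in, while this Blueprint leaves the room submixes silent.
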(event `self.ReceiveBeginPlay`
  ;[1 1 1] Turn off all sub mixes
  (`SoundSubmix.SetSubmixOutputVolume` (`self.PersistantSubmix`) 0.0)
  (for _array_element (`self.RoomSubmixes`)
    (`SoundSubmix.SetSubmixOutputVolume` _array_element 0.0))
  (for _array_element_2 (`self.AllBaseSoundscapes`)
    (`GameplayStatics.PlaySound2D` _array_element_2 1.0 1.0 0.0 null null))
  (bind (_direction _fadein) (`Timeline|Timeline` :!via `PlayFromStart`)
    (:`Update`
      (`SoundSubmix.SetSubmixOutputVolume` (`self.PersistantSubmix`) _fadein))))

(fn `UserConstructionScript`)