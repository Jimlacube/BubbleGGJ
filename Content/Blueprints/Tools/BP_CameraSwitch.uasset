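; BP_CameraSwitch is a trigger volume that moves the view to a room's camera when the player bubble enters its box.
; On overlap it skips the switch if the current camera location already matches NewCamera's.
; Otherwise it blends the view target to NewCamera with a cubic ease and tells BP_GameMode to change to the assigned Room.
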(event `self.Box.OnComponentBeginOverlap`
  (params (OverlappedComponent :type "PrimitiveComponent Object Reference") (OtherActor :type "Actor Object Reference") (OtherComp :type "PrimitiveComponent Object Reference") (OtherBodyIndex :type Integer) (bFromSweep :type Boolean) (SweepResult :type "HitResult Structure (by ref)"))
  (bind _returnvalue (`GameplayStatics.GetPlayerController` 0))
  (bind _newcamera (`self.NewCamera`))
  (cast `/Game/Blueprints/Core/BP_PlayerBubble` OtherActor)
  (if (not (== (`self.K2_GetActorLocation` _newcamera) (`PlayerCameraManager.GetCameraLocation` (`PlayerController.PlayerCameraManager` _returnvalue))))
    (`PlayerController.SetViewTargetWithBlend` _returnvalue _newcamera 1.0 "VTBlend_Cubic" 0.0 false)
    (bind _asbp_game_mode (cast `/Game/Blueprints/Core/BP_GameMode` (`GameplayStatics.GetGameMode`)))
    (`/Game/Blueprints/Core/BP_GameMode.ChangeRoom` _asbp_game_mode (`self.Room`) false)))

(fn `UserConstructionScript`)