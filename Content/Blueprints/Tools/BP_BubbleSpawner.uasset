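; BP_BubbleSpawner is an actor that periodically emits physics-driven bubbles from its own location.
; On BeginPlay it starts a looping timer that spawns a half-scale BP_Bubble every couple of seconds, ignoring collisions at the spawn point.
; Each bubble's sphere switches to physics simulation with physics-only collision and gets a random-direction velocity impulse scaled by BubbleSpawnForce.
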(event `self.ReceiveBeginPlay`
  (`KismetSystemLibrary.K2_SetTimerDelegate` (delegate `SpawnBubble`) 2.0 true true))

(event `SpawnBubble`
  (bind _returnvalue (`|SpawnActorFromClass` "/Game/Blueprints/Projectile/BP_Bubble.BP_Bubble_C" (`KismetMathLibrary.MakeTransform` (`self.K2_GetActorLocation`) (struct) (0.5 0.5 0.5)) "AlwaysSpawn" "MultiplyWithRoot" null null))
  (bind _sphere (`/Game/Blueprints/Projectile/BP_Bubble.Sphere` _returnvalue))
  (`PrimitiveComponent.SetSimulatePhysics` _sphere true)
  (`PrimitiveComponent.SetCollisionEnabled` _sphere "PhysicsOnly")
  (`PrimitiveComponent.AddImpulse` _sphere (* (`KismetMathLibrary.RandomUnitVector`) (`self.BubbleSpawnForce`)) "None" true))

(fn `UserConstructionScript`)