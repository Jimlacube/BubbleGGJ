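; BP_Bubble is a bubble actor that the player's bubble can absorb on contact.
; One second after BeginPlay it allows absorption and enables query and physics collision on its Sphere.
; An overlap with BP_PlayerBubble then calls GainBubble on it, flags the bubble as absorbed and destroys it.
; If destroyed without being absorbed, it plays a pop sound at its location.
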(event `self.ReceiveBeginPlay`
  (`KismetSystemLibrary.Delay` 1.0)
  (set `self.AllowAbsorb` true)
  (`PrimitiveComponent.SetCollisionEnabled` (`self.Sphere`) "QueryAndPhysics"))

(event `self.ReceiveDestroyed`
  ;[1 1 1] Destroyed
  (if (not (`self.HasBeenAbsorbed`))
    (`GameplayStatics.PlaySoundAtLocation` "/Game/Audio/Cues/SFX/CUE_Pop.CUE_Pop" (`self.K2_GetActorLocation`) (struct) 1.0 1.0 0.0 "/Game/Audio/Atten_Default.Atten_Default" null null null)))

(event `self.Sphere.OnComponentBeginOverlap`
  (params (OverlappedComponent :type "PrimitiveComponent Object Reference") (OtherActor :type "Actor Object Reference") (OtherComp :type "PrimitiveComponent Object Reference") (OtherBodyIndex :type Integer) (bFromSweep :type Boolean) (SweepResult :type "HitResult Structure (by ref)"))
  (if (`self.AllowAbsorb`)
    (bind _asbp_player_bubble (cast `/Game/Blueprints/Core/BP_PlayerBubble` OtherActor))
    (`/Game/Blueprints/Core/BP_PlayerBubble.GainBubble` _asbp_player_bubble false)
    (set `self.HasBeenAbsorbed` true)
    (`self.K2_DestroyActor`)))

(fn `UserConstructionScript`)